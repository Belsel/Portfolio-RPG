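; BP_Proyectile is a projectile actor for abilities that launches itself when play begins.
; A PhysicProjectile flag picks the motion: physics simulation on the Collision component with a rotated velocity-change impulse, or ProjectileMovement set to the local-space InitialVelocity.
; The construction script enables physics from that flag, and a Collision hit destroys the actor when DeadOnImpact is set.
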(event OnComponentHit(Collision)
  (params (HitComponent :type Primitive%20Component%20Object%20Reference) (OtherActor :type Actor%20Object%20Reference) (OtherComp :type Primitive%20Component%20Object%20Reference) (NormalImpulse :type Vector :default "0, 0, 0") (Hit :type Hit%20Result%20Structure%20%28by%20ref%29))
  (if (Variables|Default|GetDeadOnImpact)
    (Actor|DestroyActor)))

(event EventBeginPlay
  (bind _initial_velocity (Variables|Default|GetInitial%20Velocity))
  (if (Variables|Default|GetPhysic%20projectile)
    (Physics|AddImpulse (Variables|Default|GetCollision) (Math|Vector|RotateVector _initial_velocity (Transformation|GetActorRotation)) "None" true)
    (else
      (Game|Components|ProjectileMovement|SetVelocityinLocalSpace (Variables|Default|GetProjectileMovement) _initial_velocity))))

(event Collision|EventActorBeginOverlap
  (params (OtherActor :type Actor%20Object%20Reference)))

(event EventTick
  (params (DeltaSeconds :type Float%20%28single-precision%29)))

(fn ConstructionScript
  (Physics|SetSimulatePhysics (Variables|Default|GetCollision) (Variables|Default|GetPhysic%20projectile)))